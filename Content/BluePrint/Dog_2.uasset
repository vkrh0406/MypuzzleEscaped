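; Dog_2 is an NPC actor that opens a chat widget when the player presses F nearby.
; Its Trigger overlap, filtered by the Player tag, stores the PChara reference, shows or hides a text render and toggles the actor's input.
; Pressing F flags the player as chatting, shows the cursor and opens an introductory widget first.
; Later presses pick one of two other widgets based on whether the player has enough coins.
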(event `self.Trigger.OnComponentBeginOverlap`
  (params (OverlappedComponent :type "PrimitiveComponent Object Reference") (OtherActor :type "Actor Object Reference") (OtherComp :type "PrimitiveComponent Object Reference") (OtherBodyIndex :type Integer) (bFromSweep :type Boolean) (SweepResult :type "HitResult Structure (by ref)"))
  (if (`self.ActorHasTag` OtherActor "Player")
    (set `self.Player` (cast `/Game/BluePrint/PChara` OtherActor :!pure true))
    (`SceneComponent.SetVisibility` (`self.TextRender`) true false)
    (`self.EnableInput` (`GameplayStatics.GetPlayerController` 0))))

(event `self.Trigger.OnComponentEndOverlap`
  (params (OverlappedComponent :type "PrimitiveComponent Object Reference") (OtherActor :type "Actor Object Reference") (OtherComp :type "PrimitiveComponent Object Reference") (OtherBodyIndex :type Integer))
  (if (`self.ActorHasTag` OtherActor "Player")
    (`SceneComponent.SetVisibility` (`self.TextRender`) false false)
    (`self.DisableInput` (`GameplayStatics.GetPlayerController` 0))))

(event `Key|F`
  (params (Key :type "Key Structure"))
  (:`Pressed`
    (set `/Game/BluePrint/PChara.Ischat` true (`self.Player`))
    (if (`self.FirstChat`)
      (if (>= (`/Game/BluePrint/PChara.Coin` (`self.Player`)) 10)
        (bind _returnvalue (`|CreateWidget` "/Game/HUD/NPC2_chat2.NPC2_chat2_C"))
        (set `self.Npc_chat` _returnvalue)
        (`UserWidget.AddToViewport` _returnvalue 0)
        (set `PlayerController.bShowMouseCursor` true (`GameplayStatics.GetPlayerController` 0))
        (else
          (bind _returnvalue_2 (`|CreateWidget` "/Game/HUD/NPC2_chat3.NPC2_chat3_C"))
          (set `self.Npc_chat` _returnvalue_2)
          (`UserWidget.AddToViewport` _returnvalue_2 0)
          (set `PlayerController.bShowMouseCursor` true (`GameplayStatics.GetPlayerController` 0))))
      (else
        (bind _returnvalue_3 (`|CreateWidget` "/Game/HUD/NPC2_chat1.NPC2_chat1_C"))
        (set `self.Npc_chat` _returnvalue_3)
        (`UserWidget.AddToViewport` _returnvalue_3 0)
        (set `PlayerController.bShowMouseCursor` true (`GameplayStatics.GetPlayerController` 0))
        (set `self.FirstChat` true)))))

(fn `UserConstructionScript`)