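; Door Blueprint that swings open and closed with sound effects, driven by Open and Close events.
; Open plays GateTimeline, whose Yaw track rotates the Door component; Close plays sound 2 and reverses the timeline.
; The timeline's Opening event track passes its playback direction as an integer to PlaySE.
; PlaySE sets the Speaker's SEType parameter to select the sound, then plays it.
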(event `Open`
  (bind (_direction _yaw) (`Timeline|GateTimeline` :!label _label)
    (:`Update`
      (`SceneComponent.K2_SetRelativeRotation` (`self.door`) (`KismetMathLibrary.MakeRotator` 0.0 0.0 _yaw) false false))
    (:`Opening`
      (`self.PlaySE` (`KismetMathLibrary.Conv_ByteToInt` _direction)))))

(event `self.ReceiveBeginPlay`)

(event `Close`
  (`self.PlaySE` 2)
  (goto _label :!via `Reverse`))

(fn `PlaySE`
  (params (SE_Type :type Integer))
  (bind _speaker (`self.Speaker`))
  (`AudioComponent.SetIntParameter` _speaker "SEType" SE_Type)
  (`AudioComponent.Play` _speaker 0.0))

(fn `UserConstructionScript`)