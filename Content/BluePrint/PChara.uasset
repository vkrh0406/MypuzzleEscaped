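; PChara is the player character Blueprint, with camera-relative walking, look input and a coin counter.
; Movement follows the camera's flattened forward and right vectors, and all movement and look input is ignored while Ischat is set.
; The first damage of any amount kills the character: it ragdolls, then after a short delay the ReStart widget and mouse cursor appear.
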(event `self.ReceiveBeginPlay`
  (set `CharacterMovementComponent.MaxWalkSpeed` (`self.GroundWalkSpeed`) (`self.CharacterMovement`)))

(event `InputAxis|Front`
  (params (AxisValue :type "Float (single-precision)"))
  (if (not (`self.Ischat`))
    (`self.AddMovementInput` (`KismetMathLibrary.Normal` (`KismetMathLibrary.MakeVector` (.x (`SceneComponent.GetForwardVector` (`self.Camera`))) (.y (`SceneComponent.GetForwardVector` (`self.Camera`))))) AxisValue)))

(event `InputAxis|Right`
  (params (AxisValue :type "Float (single-precision)"))
  (if (not (`self.Ischat`))
    (`self.AddMovementInput` (`KismetMathLibrary.Normal` (`KismetMathLibrary.MakeVector` (.x (`SceneComponent.GetRightVector` (`self.Camera`))) (.y (`SceneComponent.GetRightVector` (`self.Camera`))))) AxisValue)))

(event `InputAxis|LookUp`
  (params (AxisValue :type "Float (single-precision)"))
  (if (not (`self.Ischat`))
    (`self.AddControllerPitchInput` AxisValue)))

(event `InputAxis|LookRight`
  (params (AxisValue :type "Float (single-precision)"))
  (if (not (`self.Ischat`))
    (`self.AddControllerYawInput` AxisValue)))

(event `self.ReceiveAnyDamage`
  (params (Damage :type "Float (single-precision)") (DamageType :type "DamageType Object Reference") (InstigatedBy :type "Controller Object Reference") (DamageCauser :type "Actor Object Reference"))
  (bind _mesh (`self.Mesh`))
  (`/Engine/EditorBlueprintResources/StandardMacros.DoOnce` false
    (:`Completed`
      (`|ExecutionSequence`
        (:`then_0`
          (`KismetSystemLibrary.PrintString` "Died!")
          (`CharacterMovementComponent.DisableMovement` (`self.CharacterMovement`))
          (`PrimitiveComponent.SetCollisionProfileName` _mesh "Ragdoll")
          (`PrimitiveComponent.SetSimulatePhysics` _mesh true))
        (:`then_1`
          (`KismetSystemLibrary.Delay` 2.0)
          (bind _returnvalue (`|CreateWidget` "/Game/UI/ReStart.ReStart_C"))
          (`UserWidget.AddToViewport` _returnvalue 0)
          (set `PlayerController.bShowMouseCursor` true (`GameplayStatics.GetPlayerController` 0)))))))

(fn `AddCoin`
  (`/Engine/EditorBlueprintResources/StandardMacros.IncrementInt` (`self.Coin`)))

(fn `UserConstructionScript`)