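; Pressure switch actor that turns on when an actor tagged "Player" overlaps its BoxTrigger.
; A timeline lerps the mesh slightly downward, then calls OnTurnedOn when finished; nothing reverses it.
; In parallel, a DoOnce hides the TextRender and calls RemoveWall immediately on the first overlap, without waiting for the animation.
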(event `self.BoxTrigger.OnComponentBeginOverlap`
  (params (OverlappedComponent :type "PrimitiveComponent Object Reference") (OtherActor :type "Actor Object Reference") (OtherComp :type "PrimitiveComponent Object Reference") (OtherBodyIndex :type Integer) (bFromSweep :type Boolean) (SweepResult :type "HitResult Structure (by ref)"))
  (if (`self.ActorHasTag` OtherActor "Player")
    (`|ExecutionSequence`
      (:`then_0`
        (bind (_direction _alpha) (`Timeline|SwitchTimeline`)
          (:`Update`
            (`SceneComponent.K2_SetRelativeLocation` (`self.Mesh`) (`KismetMathLibrary.VLerp` (0.0 0.0 0.0) (0.0 0.0 -8.0) _alpha) false false))
          (:`Finished`
            (`self.OnTurnedOn`))))
      (:`then_1`
        (`/Engine/EditorBlueprintResources/StandardMacros.DoOnce` false
          (:`Completed`
            (`SceneComponent.SetVisibility` (`self.TextRender`) false false)
            (`self.RemoveWall`)))))))

(event `self.ReceiveBeginPlay`)

(fn `UserConstructionScript`)