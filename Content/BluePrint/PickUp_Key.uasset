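; Key pickup actor that grants the player Key1 when touched.
; A timeline started on BeginPlay drives the static mesh's yaw.
; Box overlap by a Player-tagged actor casts it to PChara, sets the Key1 flag, plays a coin sound and destroys the pickup.
; BeginPlay also sets a short timer for EnablePickup, which is not defined in these graphs, and overlap handling has no enable check.
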(event `self.ReceiveBeginPlay`
  (`KismetSystemLibrary.K2_SetTimer` null "EnablePickup" 0.5)
  (bind (_direction _coinyaw) (`Timeline|타임라인_0`)
    (:`Update`
      (`SceneComponent.K2_SetRelativeRotation` (`self.StaticMesh`) (`KismetMathLibrary.MakeRotator` 0.0 0.0 _coinyaw) false false))))

(event `self.Box.OnComponentBeginOverlap`
  (params (OverlappedComponent :type "PrimitiveComponent Object Reference") (OtherActor :type "Actor Object Reference") (OtherComp :type "PrimitiveComponent Object Reference") (OtherBodyIndex :type Integer) (bFromSweep :type Boolean) (SweepResult :type "HitResult Structure (by ref)"))
  (if (`self.ActorHasTag` OtherActor "Player")
    (set `/Game/BluePrint/PChara.key1` true (cast `/Game/BluePrint/PChara` OtherActor :!pure true))
    (`GameplayStatics.PlaySoundAtLocation` "/Game/Audio/Game/Ma_Sfx_Snes_Coins_3_by_Dneproman_Id-334755.Ma_Sfx_Snes_Coins_3_by_Dneproman_Id-334755" (`self.K2_GetActorLocation`))
    (`self.K2_DestroyActor`)))

(fn `UserConstructionScript`)